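; Gameplay ability that triggers the equipped weapon's alternative action for the player character.
; On action start and stop, it casts the avatar actor to PlayerCharacter and forwards the call to its weapon component's PlayAlternativeAction or StopAlternativeAction.
; It holds no action logic itself and does nothing if the cast fails or the weapon component is invalid.
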(event `self.CharacterActionStart`
  (bind _asplayer_character (cast `PlayerCharacter` (`self.GetAvatarActorFromActorInfo`)))
  (bind _returnvalue (`StalkerCharacter.GetWeaponComponent` _asplayer_character))
  (`/Engine/EditorBlueprintResources/StandardMacros.IsValid` _returnvalue
    (:`Is Valid`
      (`CharacterWeaponComponent.PlayAlternativeAction` _returnvalue))))

(event `self.CharacterActionStop`
  (bind _asplayer_character (cast `PlayerCharacter` (`self.GetAvatarActorFromActorInfo`)))
  (bind _returnvalue (`StalkerCharacter.GetWeaponComponent` _asplayer_character))
  (`/Engine/EditorBlueprintResources/StandardMacros.IsValid` _returnvalue
    (:`Is Valid`
      (`CharacterWeaponComponent.StopAlternativeAction` _returnvalue))))