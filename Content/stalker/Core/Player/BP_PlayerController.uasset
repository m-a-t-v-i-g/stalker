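; BP_PlayerController is a player controller that lets the player switch control to another pawn by looking at it and pressing the 0 key.
; The key press runs a debug-drawn line trace along the view direction, limited to Pawn objects.
; When the trace hits a pawn, the controller unpossesses its current pawn and possesses the hit one.
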(event `Key|Zero`
  (params (Key :type "Key Structure"))
  (bind (_location _rotation) (`self.GetPlayerViewPoint`))
  (:`Pressed`
    (bind (_outhit _returnvalue) (`KismetSystemLibrary.LineTraceSingleForObjects` :`Start` _location :`End` (+ _location (* (`KismetMathLibrary.Conv_RotatorToVector` _rotation) 10000.0)) :`ObjectTypes` (`|MakeArray` "ObjectTypeQuery3" :!type "EObjectTypeQuery Enum") :`DrawDebugType` "ForDuration"))
    (if _returnvalue
      (bind _aspawn (cast `Pawn` (`.HitActor` (`GameplayStatics.BreakHitResult` _outhit))))
      (`self.UnPossess`)
      (`self.Possess` _aspawn))))

(fn `UserConstructionScript`)